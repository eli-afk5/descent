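; BP_Automap is a 3D automap actor that shows the player's position and heading on a rotatable, zoomable map.
; On BeginPlay, if PlayerRef is unset, it finds BP_PawnBase, converts its mesh transform relative to the first SpawnTag actor into the scaled Player marker, then centers the SpringArm there.
; Zoom changes clamped arm length, while Pitch, Yaw, Roll and SlideHorizontal step the Map component by input sign.
; The marker never updates afterward, and SlideVertical is empty.
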(event EventBeginPlay
  (bind _player (Variables|Default|GetPlayer))
  (Variables|Default|GetPlayerRef
    (:then)
    (:else
      (bind _returnvalue (Actor|GetActorOfClass "/Game/Personal_Contents/Blueprints/BP_PawnBase.BP_PawnBase_C"))
      (Variables|Default|SetPlayerRef _returnvalue)
      (bind _outactors (Actor|GetAllActorswithTag "SpawnTag"))
      (bind _output_get (Variables|Default|SetPlayerPivot (Transformation|GetActorTransform (Utilities|Array|Get(acopy) _outactors))))
      (Transformation|SetRelativeLocation _player (* (Math|Transform|InverseTransformLocation _output_get (Transformation|GetWorldLocation (Variables|/Game/Personal_Contents/Blueprints/BP_PawnBase.BP_PawnBase_C|GetMesh (Variables|Default|GetPlayerRef)))) (Variables|Default|GetScale)) false false)
      (Transformation|SetRelativeRotation _player (Math|Rotator|MakeRotator 0.0 0.0 (.yaw (Math|Transform|InverseTransformRotation _output_get (Transformation|GetWorldRotation (Variables|/Game/Personal_Contents/Blueprints/BP_PawnBase.BP_PawnBase_C|GetMesh (Variables|Default|GetPlayerRef)))))) false false)
      (Transformation|SetWorldLocation (Variables|Default|GetSpringArm) (Transformation|GetWorldLocation _player) false false))))

(fn ConstructionScript)

(fn Zoom
  (params (Value :type Float%20%28double-precision%29))
  (bind _springarm (Variables|Default|GetSpringArm))
  (if (> Value 0.0)
    (Variables|/Script/Engine.SpringArmComponent|SetTargetArmLength _springarm (Math|Float|Clamp(Float) (- (Variables|/Script/Engine.SpringArmComponent|GetTargetArmLength _springarm) 2e+01) 4e+01 5e+02))
    (else
      (Variables|/Script/Engine.SpringArmComponent|SetTargetArmLength _springarm (Math|Float|Clamp(Float) (+ (Variables|/Script/Engine.SpringArmComponent|GetTargetArmLength _springarm) 2e+01) 4e+01 5e+02)))))

(fn Pitch
  (params (Value :type Float%20%28double-precision%29))
  (bind _map (Variables|Default|GetMap))
  (bind _maprotationdelta (Variables|Default|GetMapRotationDelta))
  (if (> Value 0.0)
    (Transformation|AddLocalRotation _map (Math|Rotator|MakeRotator 0.0 _maprotationdelta 0.0) false false)
    (else
      (Transformation|AddLocalRotation _map (Math|Rotator|MakeRotator 0.0 (* _maprotationdelta -1.0) 0.0) false false))))

(fn Yaw
  (params (Value :type Float%20%28double-precision%29))
  (bind _maprotationdelta (Variables|Default|GetMapRotationDelta))
  (bind _map (Variables|Default|GetMap))
  (bind _returnvalue (Transformation|GetWorldRotation _map))
  (if (> Value 0.0)
    (Transformation|SetWorldRotation _map (Math|Rotator|MakeRotator (.roll _returnvalue) (.pitch _returnvalue) (+ (.yaw _returnvalue) _maprotationdelta)) false false)
    (else
      (Transformation|SetWorldRotation _map (Math|Rotator|MakeRotator (.roll _returnvalue) (.pitch _returnvalue) (- (.yaw _returnvalue) _maprotationdelta)) false false))))

(fn Roll
  (params (Value :type Float%20%28double-precision%29))
  (bind _maprotationdelta (Variables|Default|GetMapRotationDelta))
  (bind _map (Variables|Default|GetMap))
  (bind _returnvalue (Transformation|GetWorldRotation _map))
  (if (> Value 0.0)
    (Transformation|SetWorldRotation _map (Math|Rotator|MakeRotator (+ (.roll _returnvalue) _maprotationdelta) (.pitch _returnvalue) (.yaw _returnvalue)) false false)
    (else
      (Transformation|SetWorldRotation _map (Math|Rotator|MakeRotator (- (.roll _returnvalue) _maprotationdelta) (.pitch _returnvalue) (.yaw _returnvalue)) false false))))

(fn SlideVertical)

(fn SlideHorizontal
  (params (Value :type Float%20%28double-precision%29))
  (bind _map (Variables|Default|GetMap))
  (bind _returnvalue (Transformation|GetWorldLocation _map))
  (if (> Value 0.0)
    (Transformation|SetWorldLocation _map (Math|Vector|MakeVector (.x _returnvalue) (- (.y _returnvalue) 2.0) (.z _returnvalue)) false false)
    (else
      (Transformation|SetWorldLocation _map (Math|Vector|MakeVector (.x _returnvalue) (+ (.y _returnvalue) 2.0) (.z _returnvalue)) false false))))