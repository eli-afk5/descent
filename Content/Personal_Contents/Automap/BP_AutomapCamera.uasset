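; BP_AutomapCamera is the automap camera actor, tracking the player from far below in world space along with a player arrow marker.
; Each Tick places the actor at an X offset from the player mesh at fixed depth, copying its rotation.
; It also moves the enlarged PlayerArrow beneath the player's current position, matching yaw.
; When the player reference is invalid, Tick looks up BP_PawnBase instead.
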(event EventTick
  (params (DeltaSeconds :type Float%20%28single-precision%29))
  (bind _playerref (Variables|Default|GetPlayerRef)
    (:then
      (Transformation|SetActorTransform (Math|Transform|MakeTransform (Math|Vector|MakeVector (- (.X (Math|Vector|BreakVector (.location (Transformation|GetWorldTransform (Variables|/Game/Personal_Contents/Blueprints/BP_PawnBase.BP_PawnBase_C|GetMesh _playerref))))) 3e+03) (.Y (Math|Vector|BreakVector (.location (Transformation|GetWorldTransform (Variables|/Game/Personal_Contents/Blueprints/BP_PawnBase.BP_PawnBase_C|GetMesh _playerref))))) -1e+04) (.rotation (Transformation|GetWorldTransform (Variables|/Game/Personal_Contents/Blueprints/BP_PawnBase.BP_PawnBase_C|GetMesh _playerref))) "1.000000,1.000000,1.000000"))
      (Transformation|SetWorldTransform (Variables|Default|GetPlayerArrow) (Math|Transform|MakeTransform (Math|Vector|MakeVector (.x (.location (Variables|/Game/Personal_Contents/Blueprints/BP_PawnBase.BP_PawnBase_C|GetCurrentPlayerTransform (Variables|Default|GetPlayerRef)))) (.y (.location (Variables|/Game/Personal_Contents/Blueprints/BP_PawnBase.BP_PawnBase_C|GetCurrentPlayerTransform (Variables|Default|GetPlayerRef)))) (- (.z (.location (Variables|/Game/Personal_Contents/Blueprints/BP_PawnBase.BP_PawnBase_C|GetCurrentPlayerTransform (Variables|Default|GetPlayerRef)))) 1.15e+04)) (Math|Rotator|MakeRotator 0.0 0.0 (.yaw (.rotation (Variables|/Game/Personal_Contents/Blueprints/BP_PawnBase.BP_PawnBase_C|GetCurrentPlayerTransform (Variables|Default|GetPlayerRef))))) "20.000000,20.000000,20.000000") false false))
    (:else
      (bind _returnvalue (Actor|GetActorOfClass "/Game/Personal_Contents/Blueprints/BP_PawnBase.BP_PawnBase_C"))
      (Variables|Default|SetPlayerRef _returnvalue))))

(fn ConstructionScript)