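; Base pawn for a six-degree-of-freedom flying ship with switchable cannons and missiles, flares, shield damage and a HUD.
; Movement events apply acceleration-based forces and torques to the physics mesh, while Tick self-levels roll, drives optional bobbing and repositions the bullet spawn point.
; Fire events spend energy or ammo to spawn projectiles there, with homing missiles locking onto enemy-tagged box-trace hits.
; Map, bomb and death are print-only stubs.
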(event Custom|SwitchCannon
  (params (NewCannon :type CannonType%20Enum :default "LASER"))
  ;[0.15 0.15 0.15 0.5] Switch weapons
  (switch Utilities|FlowControl|Switch|SwitchonCannonType NewCannon
    (:LASER
      (Variables|Default|SetCannonInUse "LASER"))
    (:VULCAN
      (if (Variables|Default|GetbHasVulcanCannon)
        (Variables|Default|SetCannonInUse "VULCAN")
        (else
          (Development|PrintString "NO VULCAN" true true "(R=1.000000,G=0.000000,B=0.000000,A=1.000000)"))))))

(event Custom|SwitchMissile
  (params (NewMissile :type MissileType%20Enum :default "CONCUSSION"))
  ;[0.15 0.15 0.15 0.5] Switch weapons
  (switch Utilities|FlowControl|Switch|SwitchonMissileType NewMissile
    (:CONCUSSION
      (if (> (Variables|Default|GetConcussionCounter) 0)
        (Variables|Default|SetMissileInUse "CONCUSSION")
        (else
          (Development|PrintString "NO CONCUSSION" true true "(R=1.000000,G=0.521141,B=0.000000,A=1.000000)"))))
    (:HOMING
      (if (> (Variables|Default|GetHomingMissilesCounter) 0)
        (Variables|Default|SetMissileInUse "HOMING")
        (else
          (Development|PrintString "NO HOMING" true true "(R=1.000000,G=0.521141,B=0.000000,A=1.000000)"))))))

(event EventDoFirePrimary
  (bind _self self)
  (bind _bulletspawnpoint (Variables|Default|GetBulletSpawnPoint))
  (bind _vulcanammocounter (Variables|Default|GetVulcanAmmoCounter))
  (bind _returnvalue (Transformation|GetRelativeTransform _bulletspawnpoint))
  (bind _returnvalue_2 (Math|Vector|GetRightVector _bulletspawnpoint))
  (bind _returnvalue_3 (Math|Vector|GetForwardVector _bulletspawnpoint))
  (bind _returnvalue_4 (* _returnvalue_2 15.0))
  ;[0.6573 4e-06 1.3e-05 0.5] TODO ATTACKS
  (switch Utilities|FlowControl|Switch|SwitchonCannonType (Variables|Default|GetCannonInUse)
    (:LASER
      (if (> (Variables|Default|GetEnergyCounter) 0)
        (for _index (range 0 1)
          (switch int _index
            (:0
              (bind _output_get (Variables|Default|SetBulletLocation (+ (.location _returnvalue) _returnvalue_4))))
            (:1
              (Variables|Default|SetBulletLocation (- (.location _returnvalue) _returnvalue_4))))
          (bind _returnvalue_5 (Game|SpawnActorfromClass "/Game/Personal_Contents/Blueprints/Projectiles/BP_ProjectileLaser.BP_ProjectileLaser_C" (Math|Transform|MakeTransform _output_get (.rotation _returnvalue) (.scale _returnvalue)) "Undefined" "MultiplyWithRoot" 0 _self))
          (Default|Fire _returnvalue_5 _returnvalue_3 3e+03))
        (Variables|Default|SetEnergyCounter (- (Variables|Default|GetEnergyCounter) 0.373))))
    (:VULCAN
      (if (> _vulcanammocounter 0)
        (bind _returnvalue_6 (Game|SpawnActorfromClass "/Game/Personal_Contents/Blueprints/Projectiles/BP_ProjectileVulcan.BP_ProjectileVulcan_C" (Transformation|GetRelativeTransform (Variables|Default|GetBulletSpawnPoint)) "Undefined" "MultiplyWithRoot" 0 _self))
        (Default|Fire _returnvalue_6 _returnvalue_3 0.0)
        (Math|Integer|DecrementInt _vulcanammocounter)))))

(event EventDoSlideHorizontal
  (params (Value :type Float%20%28single-precision%29))
  (bind _mesh (Variables|Default|GetMesh))
  ;[0.15 0.15 0.15 0.5] Movement
  (Physics|AddForce _mesh (* (* Value (Variables|Default|GetMovementSpeed)) (Math|Vector|GetRightVector _mesh)) "None" true))

(event EventDoToggleMap
  ;[0.15 0.15 0.15 0.5] Other inputs
  (Development|PrintString "Map toggle (not implemented)"))

(event EventDoSwitchView
  (bind _mesh (Variables|Default|GetMesh))
  ;[0.15 0.15 0.15 0.5] Other inputs
  (Utilities|FlowControl|FlipFlop
    (:A
      (Transformation|SetRelativeLocationAndRotation _mesh "-50.000000,0.000000,0.000000" "0.000000,180.000000,0.000000" false false))
    (:B
      (Transformation|SetRelativeLocationAndRotation _mesh "50.000000,0.000000,0.000000" "0, 0, 0" false false))))

(event EventTick
  (params (DeltaSeconds :type Float%20%28single-precision%29))
  (bind _mesh (Variables|Default|GetMesh))
  (bind _mesh_2 (Variables|Default|GetMesh))
  (bind _relativerotation (Variables|/Script/Engine.SceneComponent|GetRelativeRotation _mesh_2))
  (bind _returnvalue (Math|Float|Absolute(Float) (.roll _relativerotation)))
  (bind _returnvalue_2 (> (.roll _relativerotation) 0.0))
  (Utilities|FlowControl|Sequence
    (:then_1
      ;[0.15 0.15 0.15 0.5] Camera readjustement
      (if (and (< _returnvalue 3e+01) (> _returnvalue 5.0))
        (if _returnvalue_2
          (Class|PawnBase|DoYaw 0.5 :!label _label)
          (else
            (Class|PawnBase|DoYaw -0.5 :!label _label_2)))
        (elif (and (> _returnvalue 1.5e+02) (< _returnvalue 175.0))
          (if _returnvalue_2
            (goto _label_2)
            (else
              (goto _label))))))
    (:then_2
      ;[0.15 0.15 0.15 0.5] Bobbing movement
      (if (Variables|Default|GetBobToggle)
        (Class|PawnBase|DoSlideVertical (Variables|Default|GetBobbingValue))
        (Utilities|FlowControl|DoOnce false :!label _label_3
          (:Completed
            (Utilities|FlowControl|RetriggerableDelay 0.6)
            (Variables|Default|SetBobbingValue (* (Variables|Default|GetBobbingValue) -1.0))
            (goto _label_3 Reset)))))
    (:then_3
      (Transformation|SetRelativeLocation (Variables|Default|GetBulletSpawnPoint) (+ (Variables|/Script/Engine.SceneComponent|GetRelativeLocation _mesh) (* (Math|Vector|GetForwardVector _mesh) 7e+01)) false false))))

(event Game|Damage|EventAnyDamage
  (params (Damage :type Float%20%28single-precision%29) (DamageType :type Damage%20Type%20Object%20Reference) (InstigatedBy :type Controller%20Object%20Reference) (DamageCauser :type Actor%20Object%20Reference))
  ;[0.15 0.15 0.15 0.5] Take damage
  (bind _output_get (Variables|Default|SetShieldCounter (Math|Conversions|ToFloat(Integer) (Math|Integer|Clamp(Integer) (Math|Float|Truncate (- (Variables|Default|GetShieldCounter) Damage)) 0 200))))
  (if (<= _output_get 0)
    (Development|PrintString "Death")))

(event EventBeginPlay
  (bind _returnvalue (UserInterface|CreateWidget "/Game/Personal_Contents/UI/WB_HUD.WB_HUD_C" (Game|GetPlayerController 0)))
  (UserInterface|Viewport|AddtoViewport _returnvalue 0)
  (Variables|/Game/Personal_Contents/UI/WB_HUD.WB_HUD_C|SetPlayerRef _returnvalue self))

(event EventDoSlideVertical
  (params (Value :type Float%20%28single-precision%29))
  (bind _mesh (Variables|Default|GetMesh))
  ;[0.15 0.15 0.15 0.5] Movement
  (Variables|Default|SetIsRotating true)
  (Physics|AddForce _mesh (* (* Value (Variables|Default|GetMovementSpeed)) (Math|Vector|GetUpVector _mesh)) "None" true)
  (Variables|Default|SetIsRotating false))

(event EventDoAccelerate
  (params (Value :type Float%20%28single-precision%29))
  (bind _mesh (Variables|Default|GetMesh))
  ;[0.15 0.15 0.15 0.5] Movement
  (Physics|AddForce _mesh (* (* Value (Variables|Default|GetMovementSpeed)) (Math|Vector|GetForwardVector _mesh)) "None" true))

(event EventDoYaw
  (params (Value :type Float%20%28single-precision%29))
  (bind _mesh (Variables|Default|GetMesh))
  ;[0.15 0.15 0.15 0.5] Movement
  (Class|PrimitiveComponent|AddTorqueinDegrees _mesh (* (* Value (Variables|Default|GetRotationSpeed)) (Math|Vector|GetForwardVector _mesh)) "None" true))

(event EventDoPitch
  (params (Value :type Float%20%28single-precision%29))
  (bind _mesh (Variables|Default|GetMesh))
  ;[0.15 0.15 0.15 0.5] Movement
  (Class|PrimitiveComponent|AddTorqueinDegrees _mesh (* (* Value (Variables|Default|GetRotationSpeed)) (Math|Vector|GetRightVector _mesh)) "None" true))

(event EventDoRoll
  (params (Value :type Float%20%28single-precision%29))
  (bind _mesh (Variables|Default|GetMesh))
  ;[0.15 0.15 0.15 0.5] Movement
  (Class|PrimitiveComponent|AddTorqueinDegrees _mesh (* (* Value (Variables|Default|GetRotationSpeed)) (Math|Vector|GetUpVector _mesh)) "None" true))

(event EventDoFireSecondary
  (bind _self self)
  (bind _concussioncounter (Variables|Default|GetConcussionCounter))
  (bind _bulletspawnpoint (Variables|Default|GetBulletSpawnPoint))
  (bind _homingmissilescounter (Variables|Default|GetHomingMissilesCounter))
  (bind _bulletspawnpoint_2 (Variables|Default|GetBulletSpawnPoint))
  (bind _returnvalue (Math|Vector|GetForwardVector _bulletspawnpoint))
  (bind _returnvalue_2 (Transformation|GetRelativeTransform _bulletspawnpoint))
  (bind _returnvalue_3 (Math|Vector|GetRightVector _bulletspawnpoint))
  (bind _returnvalue_4 (Transformation|GetRelativeTransform _bulletspawnpoint_2))
  (bind _returnvalue_5 (Math|Vector|GetRightVector _bulletspawnpoint_2))
  (bind _returnvalue_6 (* _returnvalue_3 15.0))
  (bind _returnvalue_7 (* _returnvalue_5 15.0))
  ;[0.6573 4e-06 1.3e-05 0.5] TODO ATTACKS
  (switch Utilities|FlowControl|Switch|SwitchonMissileType (Variables|Default|GetMissileInUse)
    (:CONCUSSION
      (if (> _concussioncounter 0)
        (Utilities|FlowControl|FlipFlop
          (:A
            (bind _output_get (Variables|Default|SetMissileLocation (+ (.location _returnvalue_4) _returnvalue_7))))
          (:B
            (Variables|Default|SetMissileLocation (- (.location _returnvalue_4) _returnvalue_7))))
        (bind _returnvalue_8 (Game|SpawnActorfromClass "/Game/Personal_Contents/Blueprints/Projectiles/BP_ProjectileConcussion.BP_ProjectileConcussion_C" (Math|Transform|MakeTransform _output_get (.rotation _returnvalue_4) (.scale _returnvalue_4)) "Undefined" "MultiplyWithRoot" 0 _self))
        (Default|Fire _returnvalue_8 (Math|Vector|GetForwardVector _bulletspawnpoint_2) 3e+03)
        (Math|Integer|DecrementInt _concussioncounter)))
    (:HOMING
      (if (> _homingmissilescounter 0)
        (Utilities|FlowControl|FlipFlop
          (:A
            (bind _output_get_2 (Variables|Default|SetMissileLocation (+ (.location _returnvalue_2) _returnvalue_6))))
          (:B
            (Variables|Default|SetMissileLocation (- (.location _returnvalue_2) _returnvalue_6))))
        (bind _returnvalue_9 (Game|SpawnActorfromClass "/Game/Personal_Contents/Blueprints/Projectiles/BP_ProjectileHoming.BP_ProjectileHoming_C" (Math|Transform|MakeTransform _output_get_2 (.rotation _returnvalue_2) (.scale _returnvalue_2)) "Undefined" "MultiplyWithRoot" 0 _self))
        (Default|Fire _returnvalue_9 _returnvalue 1e+03)
        (Math|Integer|DecrementInt _homingmissilescounter
          (:%20%20
            (bind _outhit (Collision|BoxTraceByChannel (+ (.location _returnvalue_2) (* _returnvalue 3e+02)) (+ (.location _returnvalue_2) (* _returnvalue 3e+03)) "120.000000,120.000000,120.000000" (.rotation _returnvalue_2) "TraceTypeQuery1" false 0 "ForDuration"))
            (if (Utilities|IsValid (.hitactor _outhit))
              (if (Actor|ActorHasTag (.hitactor _outhit) "enemy")
                (Variables|/Script/Engine.ProjectileMovementComponent|SetHomingTargetComponent (Variables|/Game/Personal_Contents/Blueprints/Projectiles/BP_ProjectileBase.BP_ProjectileBase_C|GetProjectileMovement _returnvalue_9) (.hitcomponent _outhit))
                (Development|PrintString "target set")))))))))

(event EventDoFireFlare
  (bind _bulletspawnpoint (Variables|Default|GetBulletSpawnPoint))
  ;[0.6573 4e-06 1.3e-05 0.5] TODO ATTACKS
  (if (> (Variables|Default|GetEnergyCounter) 0)
    (bind _returnvalue (Game|SpawnActorfromClass "/Game/Personal_Contents/Blueprints/Projectiles/BP_ProjectileFlare.BP_ProjectileFlare_C" (Transformation|GetRelativeTransform _bulletspawnpoint) "Undefined" "MultiplyWithRoot" 0 self))
    (Default|Fire _returnvalue (Math|Vector|GetForwardVector _bulletspawnpoint) 3e+03)
    (Variables|Default|SetEnergyCounter (- (Variables|Default|GetEnergyCounter) 0.373))))

(event EventDoDropBomb
  (Development|PrintString "Unused" true true "(R=0.394859,G=0.000000,B=1.000000,A=1.000000)"))

(event Input|KeyboardEvents|DebugKeyEnter
  (params (Key :type Key%20Structure :default "None") (ActionValue :type Input%20Action%20Value%20Structure))
  ;[0.15 0.15 0.15 0.5] Bobbing movement
  (:Pressed
    (Utilities|FlowControl|FlipFlop
      (:A
        (Variables|Default|SetBobToggle false)
        (Development|PrintString "Bob deactivated" true true "(R=1.000000,G=0.000000,B=0.000000,A=1.000000)"))
      (:B
        (Variables|Default|SetBobToggle true)
        (Development|PrintString "Bob activated")))))

(fn ConstructionScript)