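; Player controller for the ship that translates Enhanced Input actions into Do/Switch calls on the possessed BP_PawnBase.
; Handles flight, view and map toggles, weapon selection, flares and bombs.
; A slide toggle turns pitch and roll input into vertical and horizontal strafing, alongside a separate two-axis slide action.
; DoOnce gates with retriggerable delays throttle firing, with the primary rate depending on the cannon in use.
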(event Input|EnhancedActionEvents|EnhancedInputActionIA_Accelerate
  (params (ActionValue :type Float%20%28double-precision%29) (ElapsedSeconds :type Float%20%28double-precision%29) (TriggeredSeconds :type Float%20%28double-precision%29) (InputAction :type Input%20Action%20Object%20Reference :default "/Game/Personal_Contents/Input/Actions/IA_Accelerate.IA_Accelerate"))
  ;[0.15 0.15 0.15 0.5] Movement
  (Class|PawnBase|DoAccelerate (Variables|Default|GetPlayerRef) ActionValue))

(event Input|EnhancedActionEvents|EnhancedInputActionIA_Pitch
  (params (ActionValue :type Float%20%28double-precision%29) (ElapsedSeconds :type Float%20%28double-precision%29) (TriggeredSeconds :type Float%20%28double-precision%29) (InputAction :type Input%20Action%20Object%20Reference :default "/Game/Personal_Contents/Input/Actions/IA_Pitch.IA_Pitch"))
  (bind _playerref (Variables|Default|GetPlayerRef))
  ;[0.15 0.15 0.15 0.5] Movement
  (if (Variables|Default|GetIsSliding)
    (Class|PawnBase|DoSlideVertical _playerref ActionValue)
    (else
      (Class|PawnBase|DoPitch _playerref ActionValue))))

(event Input|EnhancedActionEvents|EnhancedInputActionIA_DropBomb
  (params (ActionValue :type Boolean) (ElapsedSeconds :type Float%20%28double-precision%29) (TriggeredSeconds :type Float%20%28double-precision%29) (InputAction :type Input%20Action%20Object%20Reference :default "/Game/Personal_Contents/Input/Actions/IA_DropBomb.IA_DropBomb"))
  ;[0.15 0.15 0.15 0.5] Attacks
  (:Started
    (Class|PawnBase|DoDropBomb (Variables|Default|GetPlayerRef))))

(event Input|EnhancedActionEvents|EnhancedInputActionIA_Map
  (params (ActionValue :type Boolean) (ElapsedSeconds :type Float%20%28double-precision%29) (TriggeredSeconds :type Float%20%28double-precision%29) (InputAction :type Input%20Action%20Object%20Reference :default "/Game/Personal_Contents/Input/Actions/IA_Map.IA_Map"))
  ;[0.15 0.15 0.15 0.5] Other inputs
  (:Started
    (Class|PawnBase|DoToggleMap (Variables|Default|GetPlayerRef))))

(event Input|EnhancedActionEvents|EnhancedInputActionIA_UseLaser
  (params (ActionValue :type Boolean) (ElapsedSeconds :type Float%20%28double-precision%29) (TriggeredSeconds :type Float%20%28double-precision%29) (InputAction :type Input%20Action%20Object%20Reference :default "/Game/Personal_Contents/Input/Actions/IA_UseLaser.IA_UseLaser"))
  ;[0.15 0.15 0.15 0.5] Switch weapons
  (:Started
    (Default|SwitchCannon (Variables|Default|GetPlayerRef) "LASER")))

(event Input|EnhancedActionEvents|EnhancedInputActionIA_UseVulkan
  (params (ActionValue :type Boolean) (ElapsedSeconds :type Float%20%28double-precision%29) (TriggeredSeconds :type Float%20%28double-precision%29) (InputAction :type Input%20Action%20Object%20Reference :default "/Game/Personal_Contents/Input/Actions/IA_UseVulkan.IA_UseVulkan"))
  ;[0.15 0.15 0.15 0.5] Switch weapons
  (:Started
    (Default|SwitchCannon (Variables|Default|GetPlayerRef) "VULCAN")))

(event Input|EnhancedActionEvents|EnhancedInputActionIA_UseConcussion
  (params (ActionValue :type Boolean) (ElapsedSeconds :type Float%20%28double-precision%29) (TriggeredSeconds :type Float%20%28double-precision%29) (InputAction :type Input%20Action%20Object%20Reference :default "/Game/Personal_Contents/Input/Actions/IA_UseConcussion.IA_UseConcussion"))
  ;[0.15 0.15 0.15 0.5] Switch weapons
  (:Started
    (Default|SwitchMissile (Variables|Default|GetPlayerRef) "CONCUSSION")))

(event Input|EnhancedActionEvents|EnhancedInputActionIA_UseHoming
  (params (ActionValue :type Boolean) (ElapsedSeconds :type Float%20%28double-precision%29) (TriggeredSeconds :type Float%20%28double-precision%29) (InputAction :type Input%20Action%20Object%20Reference :default "/Game/Personal_Contents/Input/Actions/IA_UseHoming.IA_UseHoming"))
  ;[0.15 0.15 0.15 0.5] Switch weapons
  (:Started
    (Default|SwitchMissile (Variables|Default|GetPlayerRef) "HOMING")))

(event Input|EnhancedActionEvents|EnhancedInputActionIA_MapMap
  (params (ActionValue :type Boolean) (ElapsedSeconds :type Float%20%28double-precision%29) (TriggeredSeconds :type Float%20%28double-precision%29) (InputAction :type Input%20Action%20Object%20Reference :default "/Game/Personal_Contents/Automap/IA_MapMap.IA_MapMap"))
  ;[0.15 0.15 0.15 0.5] Other inputs
  (Class|PawnBase|DoToggleMap (Variables|Default|GetPlayerRef)))

(event Input|EnhancedActionEvents|EnhancedInputActionIA_Roll
  (params (ActionValue :type Float%20%28double-precision%29) (ElapsedSeconds :type Float%20%28double-precision%29) (TriggeredSeconds :type Float%20%28double-precision%29) (InputAction :type Input%20Action%20Object%20Reference :default "/Game/Personal_Contents/Input/Actions/IA_Roll.IA_Roll"))
  (bind _playerref (Variables|Default|GetPlayerRef))
  ;[0.15 0.15 0.15 0.5] Movement
  (if (Variables|Default|GetIsSliding)
    (Class|PawnBase|DoSlideHorizontal _playerref ActionValue)
    (else
      (Class|PawnBase|DoRoll _playerref ActionValue))))

(event Input|EnhancedActionEvents|EnhancedInputActionIA_Yaw
  (params (ActionValue :type Float%20%28double-precision%29) (ElapsedSeconds :type Float%20%28double-precision%29) (TriggeredSeconds :type Float%20%28double-precision%29) (InputAction :type Input%20Action%20Object%20Reference :default "/Game/Personal_Contents/Input/Actions/IA_Yaw.IA_Yaw"))
  ;[0.15 0.15 0.15 0.5] Movement
  (Class|PawnBase|DoYaw (Variables|Default|GetPlayerRef) ActionValue))

(event Input|EnhancedActionEvents|EnhancedInputActionIA_SlideToggle
  (params (ActionValue :type Boolean) (ElapsedSeconds :type Float%20%28double-precision%29) (TriggeredSeconds :type Float%20%28double-precision%29) (InputAction :type Input%20Action%20Object%20Reference :default "/Game/Personal_Contents/Input/Actions/IA_SlideToggle.IA_SlideToggle"))
  ;[0.15 0.15 0.15 0.5] Movement
  (:Triggered
    (Variables|Default|SetIsSliding true))
  (:Completed
    (Variables|Default|SetIsSliding false)))

(event Input|EnhancedActionEvents|EnhancedInputActionIA_SlideMove
  (params (ActionValue :type Vector%202D%20Structure) (ElapsedSeconds :type Float%20%28double-precision%29) (TriggeredSeconds :type Float%20%28double-precision%29) (InputAction :type Input%20Action%20Object%20Reference :default "/Game/Personal_Contents/Input/Actions/IA_SlideMove.IA_SlideMove"))
  (bind _playerref (Variables|Default|GetPlayerRef))
  ;[0.15 0.15 0.15 0.5] Movement
  (:Triggered
    (if (not (Utilities|IsValid (stale Input|EnhancedActionEvents|EnhancedInputActionIA_SlideToggle InputAction)))
      (Variables|Default|SetIsSliding true)
      (Class|PawnBase|DoSlideVertical _playerref (.y ActionValue))
      (Class|PawnBase|DoSlideHorizontal _playerref (.x ActionValue))))
  (:Completed
    (Variables|Default|SetIsSliding false)))

(event Input|EnhancedActionEvents|EnhancedInputActionIA_ViewSwitch
  (params (ActionValue :type Boolean) (ElapsedSeconds :type Float%20%28double-precision%29) (TriggeredSeconds :type Float%20%28double-precision%29) (InputAction :type Input%20Action%20Object%20Reference :default "/Game/Personal_Contents/Input/Actions/IA_ViewSwitch.IA_ViewSwitch"))
  ;[0.15 0.15 0.15 0.5] Other inputs
  (:Started
    (Class|PawnBase|DoSwitchView (Variables|Default|GetPlayerRef))))

(event Input|EnhancedActionEvents|EnhancedInputActionIA_FirePrimary
  (params (ActionValue :type Boolean) (ElapsedSeconds :type Float%20%28double-precision%29) (TriggeredSeconds :type Float%20%28double-precision%29) (InputAction :type Input%20Action%20Object%20Reference :default "/Game/Personal_Contents/Input/Actions/IA_FirePrimary.IA_FirePrimary"))
  (bind _playerref (Variables|Default|GetPlayerRef))
  ;[0.15 0.15 0.15 0.5] Attacks
  (Utilities|FlowControl|DoOnce false :!label _label
    (:Completed
      (Class|PawnBase|DoFirePrimary _playerref)
      (switch Utilities|FlowControl|Switch|SwitchonCannonType (Variables|/Script/Descent.PawnBase|GetCannonInUse _playerref)
        (:LASER
          (Utilities|FlowControl|RetriggerableDelay 0.3)
          (goto _label Reset))
        (:VULCAN
          (Utilities|FlowControl|RetriggerableDelay 0.001)
          (goto _label Reset))))))

(event Input|EnhancedActionEvents|EnhancedInputActionIA_FireSecondary
  (params (ActionValue :type Boolean) (ElapsedSeconds :type Float%20%28double-precision%29) (TriggeredSeconds :type Float%20%28double-precision%29) (InputAction :type Input%20Action%20Object%20Reference :default "/Game/Personal_Contents/Input/Actions/IA_FireSecondary.IA_FireSecondary"))
  ;[0.15 0.15 0.15 0.5] Attacks
  (Utilities|FlowControl|DoOnce false :!label _label
    (:Completed
      (Class|PawnBase|DoFireSecondary (Variables|Default|GetPlayerRef))
      (Utilities|FlowControl|RetriggerableDelay 0.3)
      (goto _label Reset))))

(event Input|EnhancedActionEvents|EnhancedInputActionIA_FireFlare
  (params (ActionValue :type Boolean) (ElapsedSeconds :type Float%20%28double-precision%29) (TriggeredSeconds :type Float%20%28double-precision%29) (InputAction :type Input%20Action%20Object%20Reference :default "/Game/Personal_Contents/Input/Actions/IA_FireFlare.IA_FireFlare"))
  ;[0.15 0.15 0.15 0.5] Attacks
  (:Started
    (Class|PawnBase|DoFireFlare (Variables|Default|GetPlayerRef))))

(event EventBeginPlay)

(event EventTick
  (params (DeltaSeconds :type Float%20%28single-precision%29)))

(event EventPossess
  (params (PossessedPawn :type Pawn%20Object%20Reference))
  ;[0.15 0.15 0.15 0.5] Setup
  (bind _asbp_pawn_base (Utilities|Casting|CastToBP_PawnBase PossessedPawn))
  (Variables|Default|SetPlayerRef _asbp_pawn_base))

(fn ConstructionScript)