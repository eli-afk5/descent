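; BP_DestroyableDoor is a door that visibly fractures as it takes damage and opens when its health is depleted.
; It loads starting HP from a door data asset on BeginPlay, then subtracts and prints HP on every AnyDamage event.
; Hardcoded HP bands swap the static mesh between two fracture stages, and OpenDoor fires only at exactly zero HP, not below.
; A delayed debug sequence for each stage is left unconnected.
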(event Game|Damage|EventAnyDamage
  (params (Damage :type Float%20%28single-precision%29) (DamageType :type Damage%20Type%20Object%20Reference) (InstigatedBy :type Controller%20Object%20Reference) (DamageCauser :type Actor%20Object%20Reference))
  (bind _output_get (Variables|DoorSettings|SetHP (- (Variables|DoorSettings|GetHP) Damage)))
  (Development|PrintString (Utilities|String|ToString(Float) _output_get))
  (if (and (<= _output_get 6.0) (> _output_get 3.0))
    (Components|StaticMesh|SetStaticMesh (Variables|Default|GetDoorMesh) (Variables|Default|GetFirstFractureDoorMesh)))
  (if (and (<= _output_get 3.0) (> _output_get 0.0))
    (Components|StaticMesh|SetStaticMesh (Variables|Default|GetDoorMesh) (Variables|Default|GetSecondFractureDoorMesh)))
  (if (== _output_get 0.0)
    (Class|DoorBase|OpenDoor)))

(event EventBeginPlay
  (Variables|DoorSettings|SetHP (Variables|/Script/Descent.DoorsData|GetHP (Variables|Default|GetDoorDataAsset))))

(fn ConstructionScript)