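; BP_Class2Drone is an enemy drone that fires a staggered two-shot laser volley.
; FireWeapon spawns a BP_ProjectileLaser at each of two spawn points, with the second shot following after a short delay.
; Each projectile takes its damage from the enemy data asset's AttackPower and launches along the drone's forward vector at a fixed speed.
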(event EventBeginPlay)

(event Collision|EventActorBeginOverlap
  (params (OtherActor :type Actor%20Object%20Reference)))

(event EventTick
  (params (DeltaSeconds :type Float%20%28single-precision%29)))

(event EventFireWeapon
  (Utilities|FlowControl|Sequence
    (:then_0
      (bind _returnvalue (Game|SpawnActorfromClass "/Game/Personal_Contents/Blueprints/Projectiles/BP_ProjectileLaser.BP_ProjectileLaser_C" (Transformation|GetWorldTransform (Variables|Default|GetProjectileSpawnPoint)) "Undefined" "MultiplyWithRoot" 0 self))
      (Variables|/Game/Personal_Contents/Blueprints/Projectiles/BP_ProjectileBase.BP_ProjectileBase_C|SetDamage _returnvalue (Variables|/Script/Descent.EnemiesData|GetAttackPower (Variables|Default|GetEnemyDataAsset)))
      (Default|Fire _returnvalue (Transformation|GetActorForwardVector) 5e+02))
    (:then_1
      (Utilities|FlowControl|Delay 0.1)
      (bind _returnvalue_2 (Game|SpawnActorfromClass "/Game/Personal_Contents/Blueprints/Projectiles/BP_ProjectileLaser.BP_ProjectileLaser_C" (Transformation|GetWorldTransform (Variables|Default|GetProjectileSpawn2)) "Undefined" "MultiplyWithRoot" 0 self))
      (Variables|/Game/Personal_Contents/Blueprints/Projectiles/BP_ProjectileBase.BP_ProjectileBase_C|SetDamage _returnvalue_2 (Variables|/Script/Descent.EnemiesData|GetAttackPower (Variables|Default|GetEnemyDataAsset)))
      (Default|Fire _returnvalue_2 (Transformation|GetActorForwardVector) 5e+02))))

(fn ConstructionScript)