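; Base enemy Blueprint that stores its spawn origin and player pawn reference, and provides movement and firing events.
; MoveToLocation faces the destination, then runs a distance-scaled Timeline that lerps from the current location with sweep.
; FireWeapon spawns a laser projectile at the spawn point, sets its damage from the enemy data asset and launches it forward.
; Tick is empty, and the look-at-player targeting logic is left unconnected.
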(event Custom|FireWeapon
  (bind _returnvalue (Game|SpawnActorfromClass "/Game/Personal_Contents/Blueprints/Projectiles/BP_ProjectileLaser.BP_ProjectileLaser_C" (Transformation|GetWorldTransform (Variables|Default|GetProjectileSpawnPoint)) "Undefined" "MultiplyWithRoot" 0 self))
  (Variables|/Game/Personal_Contents/Blueprints/Projectiles/BP_ProjectileBase.BP_ProjectileBase_C|SetDamage _returnvalue (Variables|/Script/Descent.EnemiesData|GetAttackPower (Variables|Default|GetEnemyDataAsset)))
  (Default|Fire _returnvalue (Transformation|GetActorForwardVector) 1e+03))

(event Custom|MoveToLocation
  (params (NewLocation :type Vector) (Distance :type Float%20%28double-precision%29))
  (bind _returnvalue (Transformation|GetActorLocation))
  (Transformation|SetActorRotation (Math|Rotator|FindLookatRotation _returnvalue NewLocation))
  (Components|Timeline|SetPlayRate (Variables|Default|GetTimeline) (/ 1e+01 Distance))
  (bind _alpha (Timeline|Timeline PlayFromStart)
    (:Update
      (Transformation|SetActorLocation (Math|Vector|Lerp(Vector) _returnvalue NewLocation _alpha) true false))))

(event Collision|EventActorBeginOverlap
  (params (OtherActor :type Actor%20Object%20Reference)))

(event EventTick
  (params (DeltaSeconds :type Float%20%28single-precision%29)))

(event EventBeginPlay
  (Variables|Default|SetOrigin (Transformation|GetActorLocation))
  (bind _asbp_pawn_base (Utilities|Casting|CastToBP_PawnBase (Game|Player|GetPlayerPawn 0))
    (:then
      (Variables|Default|SetTargetRef _asbp_pawn_base))
    (:CastFailed
      (Development|PrintString "COULDNT FIND PLAYER"))))

(fn ConstructionScript)