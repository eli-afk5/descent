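; Nuclear reactor Blueprint, filed with the enemies, that acts as a damageable target.
; It loads HP from its enemy data asset on BeginPlay and subtracts incoming damage in AnyDamage.
; OnDestroyed fires only when HP lands exactly on zero, so an overshooting hit does not trigger it.
; A disconnected timed path to OnDestroyed never runs.
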(event EventBeginPlay
  (Variables|EnemySettings|SetHP (Variables|/Script/Descent.EnemiesData|GetHP (Variables|Default|GetEnemyDataAsset))))

(event Game|Damage|EventAnyDamage
  (params (Damage :type Float%20%28single-precision%29) (DamageType :type Damage%20Type%20Object%20Reference) (InstigatedBy :type Controller%20Object%20Reference) (DamageCauser :type Actor%20Object%20Reference))
  (bind _output_get (Variables|EnemySettings|SetHP (- (Variables|EnemySettings|GetHP) Damage)))
  (if (== _output_get 0.0)
    (Class|EnemyBase|OnDestroyed)))

(fn ConstructionScript)