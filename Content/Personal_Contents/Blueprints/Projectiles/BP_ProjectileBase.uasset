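; Base projectile actor that travels in a given direction and damages what it hits.
; A Fire event sets the projectile movement velocity from direction and speed, with max speed raised very high on construction.
; The bullet collision ignores the instigator.
; Its first valid hit applies damage once, prints a debug message, then destroys the actor after a DelayBetweenShots wait.
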(event OnComponentHit(BulletCollision)
  (params (HitComponent :type Primitive%20Component%20Object%20Reference) (OtherActor :type Actor%20Object%20Reference) (OtherComp :type Primitive%20Component%20Object%20Reference) (NormalImpulse :type Vector :default "0, 0, 0") (Hit :type Hit%20Result%20Structure%20%28by%20ref%29))
  (bind _instigator (Variables|Actor|GetInstigator))
  (if (!= OtherActor _instigator)
    (Utilities|FlowControl|DoOnce false
      (:Completed
        (bind _returnvalue (Game|Damage|ApplyDamage OtherActor (Variables|Default|GetDamage) 0 _instigator))
        (Development|PrintString (Utilities|String|Append "dealt " (Utilities|String|ToString(Float) _returnvalue) " damage to " (Utilities|GetDisplayName OtherActor)))
        (Utilities|FlowControl|Delay (Variables|Default|GetDelayBetweenShots))
        (Actor|DestroyActor)))))

(event Custom|Fire
  (params (Direction :type Vector) (Speed :type Float%20%28double-precision%29))
  (bind _projectilemovement (Variables|Default|GetProjectileMovement))
  (Variables|/Script/Engine.MovementComponent|SetVelocity _projectilemovement (* (Math|Vector|Normalize Direction) Speed))
  (Variables|/Script/Engine.ProjectileMovementComponent|SetInitialSpeed _projectilemovement Speed))

(event EventBeginPlay
  (Collision|IgnoreActorwhenMoving (Variables|Default|GetBulletCollision) (Variables|Actor|GetInstigator) true))

(event Collision|EventActorBeginOverlap
  (params (OtherActor :type Actor%20Object%20Reference)))

(event EventTick
  (params (DeltaSeconds :type Float%20%28single-precision%29)))

(fn ConstructionScript
  (Variables|/Script/Engine.ProjectileMovementComponent|SetMaxSpeed (Variables|Default|GetProjectileMovement) 1e+08))