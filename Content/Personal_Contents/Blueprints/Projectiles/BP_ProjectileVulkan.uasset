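; BP_ProjectileVulkan is a projectile actor that acts as an instant hitscan shot rather than a moving projectile.
; Its Fire event line-traces on the Visibility channel from the Sphere component along the given direction for a fixed range, with debug drawing enabled.
; It applies its Damage value to any valid hit actor, then destroys itself on the next tick, hit or miss.
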(event EventBeginPlay
  (|CallParentFunction) ; This node is disabled and will not be called.\nDrag off pins to build functionality.
)

(event Collision|EventActorBeginOverlap
  (params (OtherActor :type Actor%20Object%20Reference))
  (|CallParentFunction OtherActor) ; This node is disabled and will not be called.\nDrag off pins to build functionality.
)

(event EventTick
  (params (DeltaSeconds :type Float%20%28single-precision%29))
  (|CallParentFunction DeltaSeconds) ; This node is disabled and will not be called.\nDrag off pins to build functionality.
)

(event EventFire
  (params (Direction :type Vector :default "0, 0, 0") (Speed :type Float%20%28double-precision%29))
  (bind _sphere (Variables|Default|GetSphere))
  (bind _returnvalue (Transformation|GetWorldLocation _sphere))
  (bind _outhit (Collision|LineTraceByChannel _returnvalue (+ (* Direction 2e+03) _returnvalue) "TraceTypeQuery1" false 0 "ForDuration"))
  (if (Utilities|IsValid (.hitactor _outhit))
    (Game|Damage|ApplyDamage (.hitactor _outhit) (Variables|Default|GetDamage) 0 0))
  (Utilities|FlowControl|DelayUntilNextTick)
  (Actor|DestroyActor))

(fn ConstructionScript
  (|CallParentFunction))